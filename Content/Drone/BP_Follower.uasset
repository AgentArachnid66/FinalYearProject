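; BP_Follower moves itself around a Parent actor, steering its child BP_Drone away from nearby obstacles.
; Each Tick it fires debug-drawn line traces from the drone along a golden-ratio Fibonacci sphere and collects directions pointing away from hits.
; The averaged direction, dotted with drone-relative axes, nudges spherical coordinates Radius, Theta and Phi.
; UpdatePosition converts these to a point around Parent, which the actor interpolates toward.
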(event `self.ReceiveTick`
  (params (DeltaSeconds :type "Float (single-precision)"))
  (bind _returnvalue (`KismetMathLibrary.MultiplyByPi` 2.0))
  (bind _drone (`self.Drone`))
  (bind _drone_2 (`self.Drone`))
  (bind _returnvalue_2 (`self.K2_GetActorLocation` _drone))
  (bind _returnvalue_3 (* -1 _returnvalue))
  (bind _returnvalue_4 (`KismetMathLibrary.GetVectorArrayAverage` (`self.Directions`)))
  (bind _returnvalue_5 (+ (* (`KismetMathLibrary.Dot_VectorVector` (`KismetMathLibrary.GreaterGreater_VectorRotator` (`self.GetActorUpVector` _drone_2) (struct)) _returnvalue_4) -0.1) (`self.Phi`)))
  (bind _returnvalue_6 (+ (`KismetMathLibrary.Dot_VectorVector` (`KismetMathLibrary.Normal` (`KismetMathLibrary.GetDirectionUnitVector` (`self.K2_GetActorLocation` (`self.Parent`)) (`self.K2_GetActorLocation` _drone_2))) _returnvalue_4) (`self.Radius`)))
  (bind _returnvalue_7 (`KismetMathLibrary.FClamp` (+ (* (`KismetMathLibrary.Dot_VectorVector` (`KismetMathLibrary.LessLess_VectorRotator` (`self.GetActorForwardVector` _drone_2) (struct :`Yaw` 90.0)) _returnvalue_4) 0.1) (`self.Theta`)) _returnvalue_3 _returnvalue))
  (`KismetArrayLibrary.Array_Clear` (`self.Directions`))
  (bind _points_array (`self.Fibonnaci Sphere` 1000 100.0))
  (for _array_element _points_array
    (bind (_outhit _returnvalue_8) (`KismetSystemLibrary.LineTraceSingle` _returnvalue_2 (+ _returnvalue_2 _array_element) "TraceTypeQuery1" false (`|MakeArray` (`self.Drone`) :!type "Actor Object Reference") "ForOneFrame" true (struct :`R` 1.0 :`A` 1.0) (struct :`G` 0.061501 :`B` 1.0 :`A` 1.0)))
    (if _returnvalue_8
      (`KismetArrayLibrary.Array_Add` (`self.Directions`) (`KismetMathLibrary.GetDirectionUnitVector` (`.Location` (`GameplayStatics.BreakHitResult` _outhit)) (`self.K2_GetActorLocation` _drone)))))
  (set `self.Radius` _returnvalue_6)
  (set `self.Theta` _returnvalue_7)
  (set `self.Phi` (`KismetMathLibrary.FClamp` _returnvalue_5 _returnvalue_3 _returnvalue))
  (`self.K2_SetActorLocation` (`KismetMathLibrary.VInterpTo` (`self.K2_GetActorLocation`) (`self.Update Position` _returnvalue_6 _returnvalue_7 _returnvalue_5) (`GameplayStatics.GetWorldDeltaSeconds`) (`self.Interp Speed`))))

(fn `Fibonnaci Sphere`
  (params (Samples :type Integer) (`Radius Scalar` :type "Float (double-precision)" :default 1.0))
  (returns (`Points Array` :type "Array of Vector Structure"))
  (locals (Points :type "Array of Vector Structure") (`Phi ` :type "Float (double-precision)") (y :type "Float (double-precision)" :default 0.0) (`Radius ` :type "Float (double-precision)" :default 0.0) (`Theta ` :type "Float (double-precision)" :default 0.0))
  (for _index (range (+ Samples 1))
    (set `local.Theta ` (/ (`KismetMathLibrary.MultiplyByPi` (* _index 2.0)) (`self.GR`)))
    (set `local.Phi ` (`KismetMathLibrary.Acos` (- 1.0 (/ (* 2.0 (+ (`KismetMathLibrary.Conv_IntToDouble` _index) 0.5)) (`KismetMathLibrary.Conv_IntToDouble` (`local.Samples`))))))
    (`KismetArrayLibrary.Array_Add` (`local.Points`) (* (`KismetMathLibrary.MakeVector` (* (`KismetMathLibrary.Cos` (`local.Theta `)) (`KismetMathLibrary.Sin` (`local.Phi `))) (* (`KismetMathLibrary.Sin` (`local.Theta `)) (`KismetMathLibrary.Sin` (`local.Phi `))) (`KismetMathLibrary.Cos` (`local.Phi `))) (`local.Radius Scalar`))))
  (return (`local.Points`)))

(fn `Update Position`
  (params (Radius :type "Float (double-precision)") (Theta :type "Float (double-precision)") (Phi :type "Float (double-precision)"))
  (returns (ReturnValue :type "Vector Structure"))
  (bind (_returnvalue_x _returnvalue_y _returnvalue_z) (`KismetMathLibrary.BreakVector` (`self.K2_GetActorLocation` (`self.Parent`))))
  (return (`KismetMathLibrary.MakeVector` (+ (* Radius (`KismetMathLibrary.Cos` Theta) (`KismetMathLibrary.Sin` Phi)) _returnvalue_x) (+ (* Radius (`KismetMathLibrary.Sin` Theta) (`KismetMathLibrary.Sin` Phi)) _returnvalue_y) (+ (* Radius (`KismetMathLibrary.Cos` Phi)) _returnvalue_z))))

(fn `UserConstructionScript`
  (bind _asbp_drone (cast `/Game/Blueprints/BP_Drone` (`ChildActorComponent.ChildActor` (`self.ChildActor`))))
  (set `self.Drone` _asbp_drone)
  (set `self.GR` (/ (+ 1.0 (`KismetMathLibrary.Sqrt` 5.0)) 2.0)))