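; BP_Wall is an actor that bakes the material of its Wall component into a texture asset.
; The construction script creates a 512x512 render target.
; GenerateTexture clears it to black, draws the material from slot 0 into it, then writes the result to TextureTarget through the editor-only render-target-to-Texture2D conversion.
; The event graph is empty, and nothing in it calls GenerateTexture.
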(event `self.ReceiveBeginPlay`)

(fn `Generate Texture`
  (bind _rendertarget (`self.RenderTarget`))
  (`KismetRenderingLibrary.ClearRenderTarget2D` (`self.RenderTarget`))
  (`KismetRenderingLibrary.DrawMaterialToRenderTarget` _rendertarget (`PrimitiveComponent.GetMaterial` (`self.Wall`) 0))
  (`KismetRenderingLibrary.ConvertRenderTargetToTexture2DEditorOnly` _rendertarget (`self.Texture Target`)))

(fn `UserConstructionScript`
  (bind _returnvalue (`KismetRenderingLibrary.CreateRenderTarget2D` 512 512))
  (set `self.RenderTarget` _returnvalue))