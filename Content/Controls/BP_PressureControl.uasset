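; BP_PressureControl is a rotary control that turns an Interactable's orientation into a value for a Linked object.
; LocationCheck nudges Tracker yaw by the dot product of Tracker and Interactable forward vectors, wrapping negatives and clamping the result.
; It sends the normalized yaw through WindupItemMessage, displays the returned number on TextRender and prints a debug string.
; Construction caches direction vectors and draws a debug line trace.
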(event `self.Location Check`
  (bind _tracker (`self.Tracker`))
  (bind (_relativerotation_roll _relativerotation_pitch _relativerotation_yaw) (`KismetMathLibrary.BreakRotator` (`SceneComponent.RelativeRotation` _tracker)))
  (bind _returnvalue (+ _relativerotation_yaw (* 10 (`KismetMathLibrary.Dot_VectorVector` (`SceneComponent.GetForwardVector` _tracker) (`self.GetActorForwardVector` (`self.Interactable`))))))
  (bind _returnvalue_2 (`KismetMathLibrary.FClamp` (+ _returnvalue (select `bool` (< _returnvalue 0.0) :`true` 360.0 :!type "Float (single-precision)")) 0.5 320.0))
  (`SceneComponent.K2_SetRelativeRotation` _tracker (`KismetMathLibrary.MakeRotator` 0.0 0.0 _returnvalue_2) false false)
  (`KismetSystemLibrary.PrintString` "Hello")
  (bind _newvalue (message `/Game/Turret/Interact.Windup Item` (`self.Linked`) (`KismetMathLibrary.NormalizeToRange` _returnvalue_2 0.5 320.0)))
  (`TextRenderComponent.K2_SetText` (`self.TextRender`) (`KismetTextLibrary.Conv_DoubleToText` _newvalue "HalfToEven")))

(fn `UserConstructionScript`
  (bind _returnvalue (`self.K2_GetActorLocation`))
  (bind _returnvalue_2 (* (`self.GetActorRightVector`) -1))
  (set `self.InitialForwardVector` (`self.GetActorForwardVector`))
  (set `self.Offset` 0.0)
  (set `self.Initiial Right Vector` _returnvalue_2)
  (`KismetSystemLibrary.LineTraceSingle` :`Start` _returnvalue :`End` (+ (* _returnvalue_2 100) _returnvalue) :`TraceChannel` "TraceTypeQuery1" :`DrawDebugType` "ForDuration"))

(fn `WithinRange`
  (params (Value :type "Float (double-precision)") (Min :type "Float (double-precision)") (Max :type "Float (double-precision)"))
  (returns (`Within Lower` :type Boolean) (`Within Upper` :type Boolean) (`Within Range` :type Boolean))
  (bind _returnvalue (> Value Min))
  (bind _returnvalue_2 (< Value Max))
  (return _returnvalue _returnvalue_2 (and _returnvalue _returnvalue_2)))