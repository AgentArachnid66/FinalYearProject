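; BP_Control is a joystick-like control that turns an Interactable's position into turn and look-up messages for a Linked object.
; Construction links the Interactable back to it and places it at the tracker's default offset.
; When the player pawn is a LeapHandsPawn, a looping timer eases the Tracker toward the Interactable's direction, scaled to the Plane's extent.
; While active, the Tracker's normalized, centred X and Y drive those messages.
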(event `Location Check`
  (bind _tracker (`self.Tracker`))
  (bind _linked (`self.Linked`))
  (bind (_min _max) (`StaticMeshComponent.GetLocalBounds` (`self.Plane`)))
  (bind _relativelocation (`SceneComponent.RelativeLocation` _tracker))
  (bind _interactable (`self.Interactable`)
    (:`then`
      (if (`self.Active`)
        (`KismetSystemLibrary.PrintString` (`KismetStringLibrary.Conv_DoubleToString` 0.0))
        (bind (_returnvalue_x _returnvalue_y) (`KismetMathLibrary.BreakVector` (`KismetMathLibrary.VInterpTo` _relativelocation (`KismetMathLibrary.LessLess_VectorRotator` (* (`KismetMathLibrary.Normal` (- (`SceneComponent.K2_GetComponentLocation` (`/Game/Controls/BP_PlayerInteractable.StaticMesh` _interactable)) (`self.K2_GetActorLocation`))) (.x _max)) (`self.K2_GetActorRotation`)) (`GameplayStatics.GetWorldDeltaSeconds`) 15.0)))
        (`SceneComponent.K2_SetRelativeLocation` _tracker (`KismetMathLibrary.MakeVector` _returnvalue_x _returnvalue_y) false true)
        (message `/Game/Turret/Interact.Turn Item` _linked (- (`KismetMathLibrary.NormalizeToRange` (.x _relativelocation) (.x _min) (.x _max)) 0.5))
        (message `/Game/Turret/Interact.LookUp Item` _linked (- (`KismetMathLibrary.NormalizeToRange` (.y _relativelocation) (.x _min) (.x _max)) 0.5))))
    (:`else`)))

(event `self.ReceiveBeginPlay`
  (cast `/LeapMotion/Examples/LeapHandsPawn` (`GameplayStatics.GetPlayerPawn` 0))
  (bind _returnvalue (`KismetSystemLibrary.K2_SetTimerDelegate` (delegate `Location Check`) 0.1 true))
  (`KismetSystemLibrary.K2_UnPauseTimerHandle` _returnvalue))

(event `Load In`)

(event `Test`
  (bind _testbool (`self.TestBool`))
  (set `self.Active` _testbool)
  (`/Game/Turret/Interact.Activate/Deactivate` (`self.Interactable`) _testbool))

(event `/Game/Turret/Interact.Activate/Deactivate`
  (params (Value :type Boolean))
  (set `self.Active` Value)
  (`/Game/Turret/Interact.Activate/Deactivate` (`self.Interactable`) Value))

(fn `TrackToPlane`
  (bind _returnvalue (`SceneComponent.K2_GetComponentLocation` (`self.Tracker`)))
  (bind _returnvalue_2 (`SceneComponent.K2_GetComponentLocation` (`self.Tracker`)))
  (`KismetSystemLibrary.LineTraceSingle` _returnvalue (+ _returnvalue (* (0.0 0.0 -1.0) 20)) "TraceTypeQuery1")
  (`KismetSystemLibrary.LineTraceSingle` _returnvalue_2 (+ _returnvalue_2 (* (0.0 0.0 1.0) 20)) "TraceTypeQuery1"))

(fn `UserConstructionScript`
  (bind _interactable (`self.Interactable`)
    (:`then`
      (set `/Game/Controls/BP_PlayerInteractable.Linked` self _interactable)
      (`self.K2_SetActorLocation` _interactable (+ (`self.K2_GetActorLocation`) (`KismetMathLibrary.GreaterGreater_VectorRotator` (.location (`self.TrackerDefaultTransform`)) (`self.K2_GetActorRotation`))) false false))
    (:`else`)))

(fn `Windup Item`
  (params (Value :type "Float (double-precision)"))
  (returns (NewValue :type "Float (double-precision)"))
  (return 0.0))