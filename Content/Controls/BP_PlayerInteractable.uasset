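; BP_PlayerInteractable is an interactable object whose static mesh can be grabbed and released.
; An Active flag, set by Activate/Deactivate, decides whether Grab/Release snaps the mesh to a given socket or detaches it in place.
; Physics simulation turns on after attaching and off after detaching.
; Test repeats the attach toggle against TestMesh without physics changes, and Windup Item is a stub returning zero.
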(event `Test`
  (bind _staticmesh (`self.StaticMesh`))
  (if (`self.Active`)
    (`SceneComponent.K2_AttachToComponent` _staticmesh (`StaticMeshActor.StaticMeshComponent` (`self.TestMesh`)) "None" "SnapToTarget" "KeepWorld" "KeepWorld" true)
    (else
      (`SceneComponent.K2_DetachFromComponent` _staticmesh "KeepWorld" "KeepWorld" "KeepWorld" true))))

(event `/Game/Turret/Interact.Activate/Deactivate`
  (params (Value :type Boolean))
  (set `self.Active` Value))

(event `Grab/Release`
  (params (Mesh :type "SkeletalMeshComponent Object Reference") (Socket :type Name))
  (bind _staticmesh (`self.StaticMesh`))
  (if (`self.Active`)
    (`SceneComponent.K2_AttachToComponent` _staticmesh Mesh Socket "SnapToTarget" "SnapToTarget" "KeepRelative" true)
    (`PrimitiveComponent.SetSimulatePhysics` _staticmesh true)
    (else
      (`SceneComponent.K2_DetachFromComponent` _staticmesh "KeepWorld" "KeepWorld" "KeepWorld" true)
      (`PrimitiveComponent.SetSimulatePhysics` _staticmesh false))))

(fn `UserConstructionScript`)

(fn `Windup Item`
  (params (Value :type "Float (double-precision)"))
  (returns (NewValue :type "Float (double-precision)"))
  (return 0.0))