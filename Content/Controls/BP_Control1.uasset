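; BP_Control1 is a control pad that turns the position of a linked Interactable into turn and look-up messages for its Linked object.
; With a LeapHandsPawn player, a looping timer eases the Tracker toward the Interactable, clamped to the Plane's bounds, and sends normalized, centered X/Y while Active.
; Timelines animate Niagara radii and material reveals; LoadIn also moves the Interactable to the tracker's default position.
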(event `Location Check`
  (bind _tracker (`self.Tracker`))
  (bind _linked (`self.Linked`))
  (bind (_min _max) (`StaticMeshComponent.GetLocalBounds` (`self.Plane`)))
  (bind _relativelocation (`SceneComponent.RelativeLocation` _tracker))
  (`KismetSystemLibrary.PrintString` "Hello")
  (bind _interactable (`self.Interactable`)
    (:`then`
      (if (`self.Active`)
        (`SceneComponent.K2_SetRelativeLocation` _tracker (`KismetMathLibrary.VInterpTo` _relativelocation (`KismetMathLibrary.MakeVector` (`KismetMathLibrary.FClamp` (.x (- (`SceneComponent.K2_GetComponentLocation` (`/Game/Controls/BP_PlayerInteractable.StaticMesh` _interactable)) (`SceneComponent.K2_GetComponentLocation` (`self.Plane`)))) (.x _min) (.x _max)) (`KismetMathLibrary.FClamp` (.y (- (`SceneComponent.K2_GetComponentLocation` (`/Game/Controls/BP_PlayerInteractable.StaticMesh` _interactable)) (`SceneComponent.K2_GetComponentLocation` (`self.Plane`)))) (.x _min) (.x _max)) 13.0) (`GameplayStatics.GetWorldDeltaSeconds`) 15.0) false true)
        (message `/Game/Turret/Interact.Turn Item` _linked (- (`KismetMathLibrary.NormalizeToRange` (.x _relativelocation) (.x _min) (.x _max)) 0.5))
        (message `/Game/Turret/Interact.LookUp Item` _linked (- (`KismetMathLibrary.NormalizeToRange` (.y _relativelocation) (.x _min) (.x _max)) 0.5))))
    (:`else`)))

(event `self.ReceiveBeginPlay`
  (cast `/LeapMotion/Examples/LeapHandsPawn` (`GameplayStatics.GetPlayerPawn` 0))
  (`KismetSystemLibrary.K2_SetTimerDelegate` (delegate `Location Check`) 0.1 true))

(event `Load In`
  (bind _tracker (`self.Tracker`))
  (bind (_relativelocation_x _relativelocation_y _relativelocation_z) (`KismetMathLibrary.BreakVector` (`SceneComponent.RelativeLocation` _tracker)))
  (bind (_direction _newtrack_0) (`Timeline|Load In Animation` :!via `PlayFromStart`)
    (:`Update`
      (`SceneComponent.K2_SetRelativeLocation` _tracker (`KismetMathLibrary.MakeVector` 0.0 0.0 (`KismetMathLibrary.Lerp` _relativelocation_z 13.0 _newtrack_0)) false false)
      (bind _interactable (`self.Interactable`)
        (:`then`
          (`self.K2_SetActorLocation` _interactable (`KismetMathLibrary.VLerp` (`self.K2_GetActorLocation` _interactable) (+ (`self.K2_GetActorLocation`) (`self.TrackerDefaultPosition`)) _newtrack_0) false false)
          (`NiagaraComponent.SetVariableFloat` (`self.Niagara`) "Unlock Radius" (`KismetMathLibrary.Lerp` 0.0 (`self.Unlock Radius`) (`KismetMathLibrary.FClamp` (+ _newtrack_0 0.1)))))
        (:`else`)))
    (:`Finished`
      (`ActorComponent.Deactivate` (`self.Niagara`)))))

(event `/Game/Turret/Interact.Activate/Deactivate`
  (params (Value :type Boolean))
  (set `self.Active` Value)
  (`/Game/Turret/Interact.Activate/Deactivate` (`self.Interactable`) Value))

(event `Test`
  (`/Engine/EditorBlueprintResources/StandardMacros.FlipFlop`
    (:`A`
      (bind (_direction _radius) (`Timeline|Timeline_1` :!via `PlayFromStart` :!label _label)
        (:`Update`
          (`NiagaraComponent.SetVariableFloat` (`self.Niagara`) "Loading Radius" (`KismetMathLibrary.Lerp` 0.0 (`self.LoadIn Radius`) _radius)))
        (:`Finished`
          (switch `ETimelineDirection` _direction
            (:`Forward`
              (bind (_direction_2 _newtrack_0) (`Timeline|Timeline_0` :!label _label_2)
                (:`Update`
                  (`MeshComponent.SetScalarParameterValueOnMaterials` (`self.Plane`) "Percentage" _newtrack_0)
                  (`MeshComponent.SetScalarParameterValueOnMaterials` (`self.Tracker`) "Percentage" _newtrack_0)
                  (`NiagaraComponent.SetVariableFloat` (`self.Niagara`) "Radius" (`KismetMathLibrary.Lerp` 0.0 (`self.Radius`) _newtrack_0)))
                (:`Finished`
                  (switch `ETimelineDirection` _direction_2
                    (:`Backward`
                      (goto _label :!via `Reverse`))))))))))
    (:`B`
      (goto _label_2 :!via `Reverse`))))

(fn `TrackToPlane`
  (bind _returnvalue (`SceneComponent.K2_GetComponentLocation` (`self.Tracker`)))
  (bind _returnvalue_2 (`SceneComponent.K2_GetComponentLocation` (`self.Tracker`)))
  (`KismetSystemLibrary.LineTraceSingle` _returnvalue (+ _returnvalue (* (0.0 0.0 -1.0) 20)) "TraceTypeQuery1")
  (`KismetSystemLibrary.LineTraceSingle` _returnvalue_2 (+ _returnvalue_2 (* (0.0 0.0 1.0) 20)) "TraceTypeQuery1"))

(fn `UserConstructionScript`
  (bind _interactable (`self.Interactable`)
    (:`then`
      (set `/Game/Controls/BP_PlayerInteractable.Linked` self _interactable)
      (`self.K2_SetActorLocation` _interactable (`self.K2_GetActorLocation`) false false))
    (:`else`)))