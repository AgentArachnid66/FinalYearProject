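; BP_Hose is an aimable hose turret that paints a wall with its stream and gets the result scored.
; Aim and pressure inputs reshape a spline from a predicted projectile path, with spline meshes forming the visible stream.
; BP_Wall hits convert to collision UVs, where a brush material draws into a render target with pressure-driven intensity.
; A GameInstance event exports that target, posts its path to a localhost server through VaRest, and updates the score.
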(event `Calculate Score`
  (bind _returnvalue (`KismetSystemLibrary.GetProjectDirectory`))
  (bind _returnvalue_2 (subsystem `VaRestSubsystem`))
  (bind _rt_name (`self.RT_Name`))
  (bind _returnvalue_3 (`VaRestSubsystem.ConstructVaRestJsonObject` _returnvalue_2))
  (`VaRestJsonObject.SetStringField` _returnvalue_3 "imagePath" (`KismetStringLibrary.Concat_StrStr` _returnvalue _rt_name))
  (`KismetRenderingLibrary.ExportRenderTarget` "/Game/Textures/RT.RT" _returnvalue _rt_name)
  (`VaRestSubsystem.CallURL` _returnvalue_2 "http://localhost:5000/Image" "POST" "json" _returnvalue_3 (delegate `CustomEvent_0`)))

(event `CustomEvent_0`
  (params (Request :type "VaRestRequestJSON Object Reference"))
  (bind _returnvalue (`VaRestRequestJSON.GetResponseObject` Request))
  (if (`VaRestJsonObject.GetBoolField` _returnvalue "success")
    (bind _ascustom_instance (cast `/Game/CustomInstance` (`GameplayStatics.GetGameInstance`)))
    (`/Game/CustomInstance.Update Score` _ascustom_instance (`KismetMathLibrary.FTrunc` (`VaRestJsonObject.GetNumberField` _returnvalue "Score")))))

(event `self.ReceiveBeginPlay`
  (bind _ascustom_instance (cast `/Game/CustomInstance` (`GameplayStatics.GetGameInstance`)))
  (add `/Game/CustomInstance.Update Data` _ascustom_instance (delegate `Calculate Score`))
  (`self.Clear RT`)
  (bind _returnvalue (`KismetMaterialLibrary.CreateDynamicMaterialInstance` "/Game/Wall/M_Brush.M_Brush"))
  (set `self.Brush` _returnvalue))

(event `/Game/Turret/Interact.Turn Item`
  (params (Value :type "Float (single-precision)"))
  (bind _active (`self.Active`))
  (bind _defaultsceneroot (`self.DefaultSceneRoot`))
  (bind (_relativerotation_roll _relativerotation_pitch _relativerotation_yaw) (`KismetMathLibrary.BreakRotator` (`SceneComponent.RelativeRotation` _defaultsceneroot)))
  (if (or (`self.CanMove`) _active)
    (`SceneComponent.K2_AddRelativeRotation` _defaultsceneroot (`KismetMathLibrary.MakeRotator` 0.0 0.0 (`KismetMathLibrary.SelectFloat` Value 0.0 (`KismetMathLibrary.InRange_FloatFloat` (+ Value _relativerotation_yaw) -135.0 -45.0))) false false)
    (if _active :!label _label
      (`self.Move Points`))))

(event `/Game/Turret/Interact.LookUp Item`
  (params (Value :type "Float (single-precision)"))
  (bind _defaultsceneroot (`self.DefaultSceneRoot`))
  (bind (_relativerotation_roll _relativerotation_pitch _relativerotation_yaw) (`KismetMathLibrary.BreakRotator` (`SceneComponent.RelativeRotation` _defaultsceneroot)))
  (bind _returnvalue (`KismetMathLibrary.InRange_FloatFloat` (+ Value _relativerotation_pitch) -45.0 45.0))
  (if (or (`self.CanMove`) (`self.Active`))
    (`KismetSystemLibrary.PrintString` (`KismetStringLibrary.Conv_BoolToString` _returnvalue))
    (`SceneComponent.K2_AddRelativeRotation` _defaultsceneroot (`KismetMathLibrary.MakeRotator` 0.0 (`KismetMathLibrary.SelectFloat` Value 0.0 _returnvalue)) false false)
    (goto _label)))

(event `/Game/Turret/Interact.Windup Item`
  (params (Value :type "Float (single-precision)"))
  (bind _output_get (set `self.Pressure` (`KismetMathLibrary.FClamp` (+ Value (`self.Pressure`)) (`self.Min Pressure`) (`self.Max Pressure`))))
  (`KismetSystemLibrary.PrintString` (`KismetStringLibrary.Conv_DoubleToString` _output_get))
  (if (`self.Active`)
    (`self.Move Points`)))

(event `/Game/Turret/Interact.Activate/Deactivate`
  (params (Value :type Boolean))
  (`self.Toggle Active` Value))

(fn `Add Mesh`
  (locals (NewLocalVar_0 :type "ESplineCoordinateSpace Enum" :default "World"))
  (bind _spline (`self.Spline`))
  (bind _spline_2 (`self.Spline`))
  (bind _newlocalvar_0 (`local.NewLocalVar_0`))
  (bind _returnvalue_x (`KismetMathLibrary.BreakVector` (`SceneComponent.K2_GetComponentScale` _spline)))
  (`KismetArrayLibrary.Array_Clear` (`self.Meshes`))
  (bind _output_get (set `self.Section Length` (* _returnvalue_x (`self.Section`))))
  (for _index (range (+ (`KismetMathLibrary.FFloor` (/ (`SplineComponent.GetSplineLength` _spline) _output_get)) 1))
    (bind _returnvalue (`AddComponent|NODE_AddSplineMeshComponent-1`))
    (bind _returnvalue_2 (* _index _output_get))
    (bind _returnvalue_3 (* (+ _index 1) _output_get))
    (`SplineMeshComponent.SetStartAndEnd` _returnvalue (`SplineComponent.GetLocationAtDistanceAlongSpline` _spline_2 _returnvalue_2 _newlocalvar_0) (`SplineComponent.GetTangentAtDistanceAlongSpline` _spline_2 _returnvalue_2 _newlocalvar_0) (`SplineComponent.GetLocationAtDistanceAlongSpline` _spline_2 _returnvalue_3 _newlocalvar_0) (`SplineComponent.GetTangentAtDistanceAlongSpline` _spline_2 _returnvalue_3 _newlocalvar_0) true)
    (`KismetArrayLibrary.Array_Add` (`self.Meshes`) _returnvalue)))

(fn `Add Points`
  (bind _spline (`self.Spline`))
  (`SplineComponent.ClearSplinePoints` _spline true)
  (bind (_outhit _outpathpositions) (`GameplayStatics.Blueprint_PredictProjectilePath_ByTraceChannel` :`StartPos` (`SceneComponent.K2_GetComponentLocation` _spline) :`LaunchVelocity` (* (`SceneComponent.GetForwardVector` (`self.Turret`)) (`self.Pressure`)) :`ProjectileRadius` 0.3 :`DrawDebugType` "ForDuration"))
  (for (_array_element _array_index) _outpathpositions
    (if (== (mod _array_index (/ (`KismetArrayLibrary.Array_Length` _outpathpositions) (`self.Num Segments`))) 0)
      (`SplineComponent.AddSplinePoint` (`self.Spline`) _array_element "World" true))))

(fn `Clear Mesh`
  (for _array_element (`self.Meshes`)
    (`ActorComponent.K2_DestroyComponent` _array_element)))

(fn `Clear RT`
  (`KismetSystemLibrary.PrintString` "Clearing Render Target")
  (`KismetRenderingLibrary.ClearRenderTarget2D` "/Game/Textures/RT.RT"))

(fn `Draw To RT`
  (params (`UV Location` :type "LinearColor Structure"))
  (locals (`Canvas Size` :type "Float (double-precision)" :default 256.0))
  (bind (_r _g) (break `LinearColor` `UV Location`))
  (bind _brush (`self.Brush`))
  (bind _uv_locations (`self.UV Locations`))
  (bind _returnvalue (`KismetMathLibrary.MakeVector2D` _r _g))
  (`MaterialInstanceDynamic.SetVectorParameterValue` _brush "UV Transform" `UV Location`)
  (`MaterialInstanceDynamic.SetScalarParameterValue` _brush "Size" (`self.Brush Size`))
  (`MaterialInstanceDynamic.SetScalarParameterValue` _brush "Intensity" (`CurveFloat.GetFloatValue` (`self.Curve`) (`KismetMathLibrary.NormalizeToRange` (`self.Pressure`) (`self.Min Pressure`) (`self.Max Pressure`))))
  (`KismetRenderingLibrary.DrawMaterialToRenderTarget` "/Game/Textures/RT.RT" _brush)
  (if (not (`KismetArrayLibrary.Array_Contains` _uv_locations _returnvalue))
    (`KismetArrayLibrary.Array_Add` _uv_locations _returnvalue)
    (`KismetArrayLibrary.Array_Add` (`self.HitLocations`) (`|MakeJson` _r _g))))

(fn `Draw Wall`
  (params (Hit :type "HitResult Structure (by ref)") (TargetArray :type "Array of Vector Structure (by ref)") (End :type "Vector Structure"))
  (cast `/Game/Wall/BP_Wall` (`.HitActor` (`GameplayStatics.BreakHitResult` Hit)))
  (bind _outhit (`KismetSystemLibrary.LineTraceSingle` :`Start` (`|GetArrayItem` TargetArray (- (`KismetArrayLibrary.Array_Length` TargetArray) 2)) :`End` End :`TraceChannel` "TraceTypeQuery1" :`bTraceComplex` true :`DrawDebugType` "ForDuration"))
  (`self.Draw to RT` (`KismetMathLibrary.Conv_VectorToLinearColor` (`KismetMathLibrary.Conv_Vector2DToVector` (`GameplayStatics.FindCollisionUV` _outhit)))))

(fn `Move Mesh`
  (locals (NewLocalVar_1 :type "ESplineCoordinateSpace Enum" :default "Local"))
  (bind _section_length (`self.Section Length`))
  (bind _spline (`self.Spline`))
  (bind _newlocalvar_1 (`local.NewLocalVar_1`))
  (bind _relativelocation (`SceneComponent.RelativeLocation` _spline))
  (for (_array_element _array_index) (`self.Meshes`)
    (bind _returnvalue (* _array_index _section_length))
    (bind _returnvalue_2 (* (+ _array_index 1) _section_length))
    (`SplineMeshComponent.SetStartAndEnd` _array_element (+ (`SplineComponent.GetLocationAtDistanceAlongSpline` _spline _returnvalue _newlocalvar_1) _relativelocation) (`SplineComponent.GetTangentAtDistanceAlongSpline` _spline _returnvalue _newlocalvar_1) (+ (`SplineComponent.GetLocationAtDistanceAlongSpline` _spline _returnvalue_2 _newlocalvar_1) _relativelocation) (`SplineComponent.GetTangentAtDistanceAlongSpline` _spline _returnvalue_2 _newlocalvar_1) true)))

(fn `Move Points`
  (`KismetArrayLibrary.Array_Clear` (`self.Spline Positions`))
  (bind (_outhit _outpathpositions _outlasttracedestination) (`GameplayStatics.Blueprint_PredictProjectilePath_ByTraceChannel` :`StartPos` (`SceneComponent.K2_GetComponentLocation` (`self.Spline`)) :`LaunchVelocity` (* (`SceneComponent.GetForwardVector` (`self.Turret`)) (`self.Pressure`)) :`ProjectileRadius` 0.3 :`TraceChannel` "ECC_Visibility" :`bTraceComplex` true :`DrawDebugType` "ForDuration"))
  (`self.Draw Wall` _outhit _outpathpositions _outlasttracedestination)
  (for (_array_element _array_index) _outpathpositions
    (if (== (mod _array_index (/ (`KismetArrayLibrary.Array_Length` _outpathpositions) (`self.Num Segments`))) 0)
      (`KismetArrayLibrary.Array_Add` (`self.Spline Positions`) _array_element)))
  (`SplineComponent.SetSplinePoints` (`self.Spline`) (`self.Spline Positions`) "World" true)
  (`self.Move Mesh`))

(fn `Toggle Active`
  (params (Active :type Boolean))
  (bind _output_get (set `self.Active` Active))
  (`KismetSystemLibrary.PrintString` (select `bool` _output_get :`false` "Hidden" :`true` "Visible"))
  (for _array_element (`self.Meshes`)
    (`SceneComponent.SetVisibility` _array_element _output_get false)))

(fn `UserConstructionScript`
  (locals (NumSegments :type Integer))
  (`self.Add Points`)
  (`self.Add Mesh`)
  (`KismetMaterialLibrary.SetVectorParameterValue` "/Game/Wall/Wall.Wall" "Control" (`self.Member`))
  (`self.Toggle Active` false))