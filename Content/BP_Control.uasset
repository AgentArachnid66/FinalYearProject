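; BP_Control is a Leap Motion grabbable control that steers a linked object's turn and look-up.
; Grab events from LeapHandsPawn attach PlayerInteractable to the hand's wrist socket or detach it, and pass the grab state to Linked.
; A looping timer eases Tracker toward the interactable's position, clamped to Plane's bounds.
; Tracker's normalized, centered X and Y feed Linked's turn and look-up messages, making the plane a two-axis joystick.
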(event `Location Check`
  (bind _tracker (`self.Tracker`))
  (bind _linked (`self.Linked`))
  (bind (_min _max) (`StaticMeshComponent.GetLocalBounds` (`self.Plane`)))
  (bind _relativelocation (`SceneComponent.RelativeLocation` _tracker))
  (`SceneComponent.K2_SetRelativeLocation` _tracker (`KismetMathLibrary.VInterpTo` _relativelocation (`KismetMathLibrary.MakeVector` (`KismetMathLibrary.FClamp` (.x (- (`SceneComponent.K2_GetComponentLocation` (`self.Player Interactable`)) (`SceneComponent.K2_GetComponentLocation` (`self.Plane`)))) (.x _min) (.x _max)) (`KismetMathLibrary.FClamp` (.y (- (`SceneComponent.K2_GetComponentLocation` (`self.Player Interactable`)) (`SceneComponent.K2_GetComponentLocation` (`self.Plane`)))) (.y _min) (.y _max)) 245.0) (`GameplayStatics.GetWorldDeltaSeconds`) 15.0) false true)
  (message `/Game/Turret/Interact.Turn Item` _linked (- (`KismetMathLibrary.NormalizeToRange` (.x _relativelocation) (.x _min) (.x _max)) 0.5))
  (message `/Game/Turret/Interact.LookUp Item` _linked (- (`KismetMathLibrary.NormalizeToRange` (.y _relativelocation) (.y _min) (.y _max)) 0.5)))

(event `self.ReceiveBeginPlay`
  (bind _asleap_hands_pawn (cast `/LeapMotion/Examples/LeapHandsPawn` (`GameplayStatics.GetPlayerPawn` 0)))
  (add `/LeapMotion/Examples/LeapHandsPawn.Start/End Grab` _asleap_hands_pawn (delegate `Activate/Deactivate`))
  (bind _returnvalue (`KismetSystemLibrary.K2_SetTimerDelegate` (delegate `Location Check`) 0.1 true))
  (set `self.LocationTimer` _returnvalue))

(event `Activate/Deactivate`
  (params (`Hand Mesh` :type "SkeletalMeshComponent Object Reference") (`Hand Type` :type "EHandType Enum" :default "LEAP_HAND_LEFT") (Grab :type Boolean))
  (bind _player_interactable (`self.Player Interactable`))
  (message `/Game/Turret/Interact.Activate/Deactivate` (`self.Linked`) Grab)
  (if Grab
    (if true
      (`PrimitiveComponent.SetSimulatePhysics` _player_interactable false)
      (`SceneComponent.K2_AttachToComponent` _player_interactable `Hand Mesh` (select `EHandType` `Hand Type` :`LEAP_HAND_LEFT` "L_WristSocket" :`LEAP_HAND_RIGHT` "R_WristSocket" :!type "Name") "SnapToTarget" "SnapToTarget" "KeepRelative" false)
      (`KismetSystemLibrary.K2_UnPauseTimerHandle` (`self.LocationTimer`))
      (else
        (`KismetSystemLibrary.PrintString` "Hello")))
    (else
      (`SceneComponent.K2_DetachFromComponent` (`self.Player Interactable`) "KeepWorld" "KeepWorld" "KeepWorld" true)
      (`KismetSystemLibrary.PrintString` "Released"))))

(fn `TrackToPlane`
  (bind _returnvalue (`SceneComponent.K2_GetComponentLocation` (`self.Tracker`)))
  (bind _returnvalue_2 (`SceneComponent.K2_GetComponentLocation` (`self.Tracker`)))
  (`KismetSystemLibrary.LineTraceSingle` _returnvalue (+ _returnvalue (* (0.0 0.0 -1.0) 20)) "TraceTypeQuery1")
  (`KismetSystemLibrary.LineTraceSingle` _returnvalue_2 (+ _returnvalue_2 (* (0.0 0.0 1.0) 20)) "TraceTypeQuery1"))

(fn `UserConstructionScript`)